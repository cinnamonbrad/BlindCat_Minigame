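; Seeker pawn for the Blind Cat game, which tags runners by capsule hit and removes their IDs from the game state's remaining runners.
; When locally controlled, it creates a black-screen overlay holding a reference to itself, plus a minimap.
; Tick turns the minimap pointer with mesh yaw and scans all runners to update the nearest horizontal distance.
; A sphere overlap with a runner calls ShowVisualFootsteps, which is empty here.
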(event OnComponentBeginOverlap(Sphere)
  (params (OverlappedComponent :type Primitive%20Component%20Object%20Reference) (OtherActor :type Actor%20Object%20Reference) (OtherComp :type Primitive%20Component%20Object%20Reference) (OtherBodyIndex :type Integer) (bFromSweep :type Boolean) (SweepResult :type Hit%20Result%20Structure%20%28by%20ref%29))
  (Utilities|Casting|CastToBP_Runner OtherActor)
  (CallFunction|ShowVisualFootsteps))

(event OnComponentHit(CapsuleComponent)
  (params (HitComponent :type Primitive%20Component%20Object%20Reference) (OtherActor :type Actor%20Object%20Reference) (OtherComp :type Primitive%20Component%20Object%20Reference) (NormalImpulse :type Vector :default "0, 0, 0") (Hit :type Hit%20Result%20Structure%20%28by%20ref%29))
  (bind _asbp_runner (Utilities|Casting|CastToBP_Runner OtherActor))
  (bind _asblind_cat_game_state (Utilities|Casting|CastToBlindCatGameState (Game|GetGameState)))
  (Utilities|Array|RemoveItem (Variables|/Game/BlindCat_Minigame/Blueprints/BlindCatGameState.BlindCatGameState_C|GetremainingRunners _asblind_cat_game_state) (Variables|/Game/BlindCat_Minigame/Blueprints/BP_Runner.BP_Runner_C|GetrunnerId _asbp_runner)))

(event Custom|showVisualFootsteps)

(event EventBeginPlay
  (|CallParentFunction)
  (if (Pawn|IsLocallyControlled)
    (bind _asplayer_controller (Utilities|Casting|CastToPlayerController (Pawn|GetController self)))
    (bind _returnvalue (UserInterface|CreateWidget "/Game/BlindCat_Minigame/Blueprints/BlackScreen4Seeker.BlackScreen4Seeker_C" _asplayer_controller))
    (bind _output_get (Variables|Default|SetBlackScreenWidget _returnvalue))
    (Variables|/Game/BlindCat_Minigame/Blueprints/BlackScreen4Seeker.BlackScreen4Seeker_C|SetseekerRef _returnvalue self)
    (UserInterface|Viewport|AddtoPlayerScreen _output_get)
    (bind _returnvalue_2 (UserInterface|CreateWidget "/Game/BlindCat_Minigame/Blueprints/Minimap.Minimap_C" _asplayer_controller))
    (UserInterface|Viewport|AddtoPlayerScreen _returnvalue_2 1)
    (Variables|Default|SetminimapWidget _returnvalue_2)))

(event EventTick
  (params (DeltaSeconds :type Float%20%28single-precision%29))
  (bind _minimapwidget (Variables|Default|GetminimapWidget))
  (|CallParentFunction DeltaSeconds)
  (Utilities|FlowControl|Sequence
    (:then_0
      (if (!= _minimapwidget 0)
        (Default|ChangePointerAngle _minimapwidget (+ (.yaw (Transformation|GetWorldRotation (Variables|Character|GetMesh))) 9e+01))))
    (:then_1
      (bind _outactors (Actor|GetAllActorsOfClass "/Game/BlindCat_Minigame/Blueprints/BP_Runner.BP_Runner_C"))
      (Variables|Default|Settemp 1e+04)
      (for _array_element _outactors
        (Variables|Default|Settemp (Math|Float|Min(Float) (Transformation|GetHorizontalDistanceTo self _array_element) (Variables|Default|Gettemp))))
      (Variables|Default|SetdistanceNearestRunner (Variables|Default|Gettemp)))))

(fn ConstructionScript
  (|CallParentFunction))