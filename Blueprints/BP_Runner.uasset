(event OnComponentHit(CapsuleComponent)
  (params (HitComponent :type Primitive%20Component%20Object%20Reference) (OtherActor :type Actor%20Object%20Reference) (OtherComp :type Primitive%20Component%20Object%20Reference) (NormalImpulse :type Vector :default "0, 0, 0") (Hit :type Hit%20Result%20Structure%20%28by%20ref%29))
  (Utilities|Casting|CastToBP_Seeker OtherActor)
  (Utilities|FlowControl|Sequence
    (:then_0
      (if (Pawn|IsLocallyControlled)
        (bind _returnvalue (UserInterface|CreateWidget "/Game/BlindCat_Minigame/Blueprints/NotificationHUD.NotificationHUD_C"))
        (Rendering|Components|TextRender|SetText (Variables|/Game/BlindCat_Minigame/Blueprints/NotificationHUD.NotificationHUD_C|GetnotificationText _returnvalue) "You're Out!")
        (UserInterface|Viewport|AddtoPlayerScreen _returnvalue)
        (Components|Animation|PlayAnimation _returnvalue (Variables|/Game/BlindCat_Minigame/Blueprints/NotificationHUD.NotificationHUD_C|GetshowText _returnvalue) 0.0
          (:Finished
            (Widget|RemovefromParent _returnvalue)))))))

(event EventBeginPlay
  (|CallParentFunction) ; This node is disabled and will not be called.\nDrag off pins to build functionality.
)

(event EventTick
  (params (DeltaSeconds :type Float%20%28single-precision%29)))

(fn ConstructionScript
  (|CallParentFunction))